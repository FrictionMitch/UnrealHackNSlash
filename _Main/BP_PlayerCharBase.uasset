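; Base multiplayer player character Blueprint for melee combat, with a primary attack and three ability inputs.
; Inputs gated by IsAttacking call server events that only set that flag, while separate multicast events handle montage, sounds and capsule collision profile.
; Server-side melee hitbox overlaps resolve enemies through EnemyRefMessage, apply fixed damage and multicast the hit sound.
; PlayerRef returns the character itself.
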(event OnComponentBeginOverlap(MeleeHitBox)
  (params (OverlappedComponent :type Primitive%20Component%20Object%20Reference) (OtherActor :type Actor%20Object%20Reference) (OtherComp :type Primitive%20Component%20Object%20Reference) (OtherBodyIndex :type Integer) (bFromSweep :type Boolean) (SweepResult :type Hit%20Result%20Structure%20%28by%20ref%29))
  ;[1 1 1] Attack Collision / Damage
  (Networking|SwitchHasAuthority
    (:Authority
      (if true
        (bind _enemyref (Class|IEnemyAIInterface|EnemyRef(Message) OtherActor))
        (Utilities|IsValid _enemyref
          (:Is%20Valid
            (Utilities|Array|AddUnique (Variables|Default|GetHitEnemies) _enemyref)
            (bind _arrayelement (Utilities|Array|ReverseforEachLoop (Variables|Default|GetHitEnemies))
              (:LoopBody
                (Default|ReceiveDamage _arrayelement 100))
              (:Completed
                (Utilities|Array|Clear (Variables|Default|GetHitEnemies))
                (CallFunction|MultiPlayHitSound (Variables|Default|GetHitSound) (Transformation|GetActorLocation))))))))))

(event Custom|SRVR_PrimaryAttack
  ;[1 1 1] Primary Attack
  ;;[1 1 1] SRVR Call Multicast Event
  (Variables|Default|SetbIsAttacking true))

(event Custom|Multi_PrimaryAttack
  (params (Montage :type Anim%20Montage%20Object%20Reference))
  ;[1 1 1] Multicast runs animation
  (Animation|Montage|PlayMontage (Variables|Character|GetMesh) Montage 1.0 0.0 "AttackStart"
    (:OnNotifyBegin
      (Audio|PlaySoundatLocation (Variables|Default|GetAttackSound) (Transformation|GetActorLocation) "0, 0, 0" 1.0 1.0 0.0 0 0 0))))

(event Custom|SVR_AbilityThree
  ;[1 1 1] Ability Three
  (Variables|Default|SetbIsAttacking true))

(event Custom|SVR_AbilityOne
  ;[1 1 1] Ability One
  (Variables|Default|SetbIsAttacking true))

(event Custom|SVR_AbilityTwo
  ;[1 1 1] Ability Two
  (Variables|Default|SetbIsAttacking true))

(event Custom|Multi_CollisionOverlap
  (params (bIsRagdoll :type Boolean) (CollisionProfile :type Name))
  ;[1 1 1] Set Collision to Ragdoll
  (if bIsRagdoll
    (Collision|SetCollisionProfileName (Variables|Default|GetCapsuleComponent) CollisionProfile true :!class /Script/Engine.PrimitiveComponent)
    (else
      (Collision|SetCollisionProfileName (Variables|Default|GetCapsuleComponent) CollisionProfile true :!class /Script/Engine.PrimitiveComponent))))

(event Custom|Multi_PlayHitSound
  (params (HitSound :type Sound%20Cue%20Object%20Reference) (Location :type Vector))
  ;[1 1 1] Attack Collision / Damage
  (Audio|PlaySoundatLocation HitSound Location "0, 0, 0" 1.0 1.0 0.0 0 0 0))

(event EventBeginPlay)

(event Collision|EventActorBeginOverlap
  (params (OtherActor :type Actor%20Object%20Reference)))

(event EventTick
  (params (DeltaSeconds :type Float%20%28single-precision%29)))

(event Input|ActionEvents|InputActionAbilityOne
  (params (Key :type Key%20Structure :default "None"))
  ;[1 1 1] Ability One
  (:Pressed
    (if (not (Variables|Default|GetbIsAttacking))
      (CallFunction|SVRAbilityOne))))

(event Input|ActionEvents|InputActionPrimaryAttack
  (params (Key :type Key%20Structure :default "None"))
  ;[1 1 1] Primary Attack
  ;;[1 1 1] Input -> Call SRVR Event
  (:Pressed
    (if (not (Variables|Default|GetbIsAttacking))
      (CallFunction|SRVRPrimaryAttack))))

(event Input|ActionEvents|InputActionAbilityTwo
  (params (Key :type Key%20Structure :default "None"))
  ;[1 1 1] Ability Two
  (:Pressed
    (if (not (Variables|Default|GetbIsAttacking))
      (CallFunction|SVRAbilityTwo))))

(event Input|ActionEvents|InputActionAbilityThree
  (params (Key :type Key%20Structure :default "None"))
  ;[1 1 1] Ability Three
  (:Pressed
    (if (not (Variables|Default|GetbIsAttacking))
      (CallFunction|SVRAbilityThree))))

(fn ConstructionScript)

(fn PlayerRef
  (return self))