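; Player controller Blueprint that drives movement of whatever pawn it controls from the MoveForward and MoveRight axis inputs.
; Each axis event checks that the controlled pawn is valid, then adds movement input along the forward or right vector of that pawn's control rotation, scaled by the axis value.
; BeginPlay, Tick and the construction script hold no logic.
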(event EventBeginPlay)

(event EventTick
  (params (DeltaSeconds :type Float%20%28single-precision%29)))

(event Input|AxisEvents|InputAxisMoveForward
  (params (AxisValue :type Float%20%28single-precision%29))
  (bind _returnvalue (Pawn|GetControlledPawn))
  (Utilities|IsValid _returnvalue
    (:Is%20Valid
      (Pawn|Input|AddMovementInput _returnvalue (Math|Vector|GetForwardVector (Pawn|GetControlRotation _returnvalue :!class /Script/Engine.Pawn)) AxisValue false))))

(event Input|AxisEvents|InputAxisMoveRight
  (params (AxisValue :type Float%20%28single-precision%29))
  (bind _returnvalue (Pawn|GetControlledPawn))
  (Utilities|IsValid _returnvalue
    (:Is%20Valid
      (Pawn|Input|AddMovementInput _returnvalue (Math|Vector|GetRightVector (Pawn|GetControlRotation _returnvalue :!class /Script/Engine.Pawn)) AxisValue false))))

(fn ConstructionScript)