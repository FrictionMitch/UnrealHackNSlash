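; Base enemy character that chases a target player and plays a worm attack montage when in range.
; SetNewTarget locks the first target, enters combat, switches to walking speed via a movement-state function and starts AI MoveTo.
; Reaching the target enables Tick, which eases yaw toward it, and plays the montage once.
; Damage handling and montage completion only print debug strings.
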(event Custom|ReceiveDamage
  (params (Damage :type Integer))
  (Development|PrintString (Utilities|String|ToString(Integer) Damage)))

(event Custom|SetNewTarget
  (params (Player :type BP%20Player%20Char%20Base%20Object%20Reference))
  (Utilities|IsValid (Variables|Default|GetTarget)
    (:Is%20Not%20Valid
      (Variables|Default|SetTarget Player)
      (Variables|Default|SetbInCombat true)
      (CallFunction|FMovementState "Walking")
      (CallFunction|ChasePlayer))))

(event Custom|ChasePlayer
  (if (Variables|Default|GetbInCombat)
    (AI|AIMoveTo self "0, 0, 0" (Variables|Default|GetTarget) (Variables|Default|GetAcceptanceRadius) false
      (:OnSuccess
        (Development|PrintString "WIthin Range")
        (CallFunction|RotateTowardsPlayer)
        (CallFunction|AttackPlayerMontage)))))

(event Custom|RotateTowardsPlayer
  (Actor|Tick|SetActorTickEnabled true))

(event Custom|AttackPlayerMontage
  (Animation|Montage|PlayMontage (Variables|Character|GetMesh) "/Game/_AI/WormAttack_Montage.WormAttack_Montage"
    (:OnCompleted
      (Development|PrintString "Worm Fired"))))

(event EventBeginPlay
  (CallFunction|FMovementState "Idle"))

(event Collision|EventActorBeginOverlap
  (params (OtherActor :type Actor%20Object%20Reference)))

(event EventTick
  (params (DeltaSeconds :type Float%20%28single-precision%29))
  (if (Variables|Default|GetbInCombat)
    (Transformation|SetActorRotation (Math|Interpolation|RInterpTo (Transformation|GetActorRotation) (Math|Rotator|MakeRotator 0.0 0.0 (.yaw (Math|Rotator|FindLookatRotation (Transformation|GetActorLocation) (Transformation|GetActorLocation (Variables|Default|GetTarget))))) 0.5 0.05))))

(fn ConstructionScript)

(fn FMovementState
  (params (State :type EMovementState%20Enum :default "Idle"))
  (bind _charactermovement (Variables|Character|GetCharacterMovement))
  (switch Utilities|FlowControl|Switch|SwitchonEMovementState State
    (:Idle
      (Variables|/Script/Engine.CharacterMovementComponent|SetMaxWalkSpeed _charactermovement (Variables|Default|GetIdleSpeed)))
    (:Walking
      (Variables|/Script/Engine.CharacterMovementComponent|SetMaxWalkSpeed _charactermovement (Variables|Default|GetWalkSpeed)))
    (:Sprinting
      (Variables|/Script/Engine.CharacterMovementComponent|SetMaxWalkSpeed _charactermovement (Variables|Default|GetSprintSpeed)))))

(fn EnemyRef
  (return self))